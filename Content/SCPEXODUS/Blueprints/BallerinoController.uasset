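; BallerinoController is an AI controller for the Ballerino character that handles sight detection of the player.
; When perception updates, it loops over currently seen actors and casts them to BP_Player_Jack, breaking on a match.
; It writes that player reference to the TargetActor blackboard key and prints a debug detection message.
; Nothing here clears the key when sight is lost, and BeginPlay and Tick are unused.
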(event OnPerceptionUpdated(AIPerception)
  (params (UpdatedActors :type Array%20of%20Actor%20Object%20References))
  (if (> (Utilities|Array|Length (Class|AIPerceptionComponent|GetCurrentlyPerceivedActors (Variables|Default|GetAIPerception) "/Script/AIModule.AISense_Sight")) 0)
    (bind _array_element (Utilities|Array|ForEachLoopwithBreak (Class|AIPerceptionComponent|GetCurrentlyPerceivedActors (Variables|Default|GetAIPerception) "/Script/AIModule.AISense_Sight") :!label _label)
      (:LoopBody
        (bind _asbp_player_jack (Utilities|Casting|CastToBP_Player_Jack _array_element))
        (goto _label Break))
      (:Completed
        (AI|Components|Blackboard|SetValueasObject (Variables|Default|GetBlackboard) (Utilities|Name|MakeLiteralName "TargetActor") _asbp_player_jack)
        (Development|PrintString "Ballerino has DETECTED")))))

(event EventBeginPlay)

(event EventTick
  (params (DeltaSeconds :type Float%20%28single-precision%29)))

(fn ConstructionScript)