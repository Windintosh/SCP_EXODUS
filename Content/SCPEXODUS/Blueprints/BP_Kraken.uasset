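; BP_Kraken is an AI-driven Kraken character that can take damage and die.
; On BeginPlay it runs the BT_Kraken behavior tree unless already dead.
; AnyDamage subtracts from HP and prints a debug readout.
; At zero HP it stops the AI logic and movement, then a DoOnce plays the death sound and animation and destroys the actor after a delay.
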(event EventBeginPlay
  (if (not (Variables|Default|GetIsDead))
    (AI|RunBehaviorTree (AI|GetAIController self) "/Game/SCPEXODUS/Blueprints/BT_Kraken.BT_Kraken")))

(event Collision|EventActorBeginOverlap
  (params (OtherActor :type Actor%20Object%20Reference)))

(event EventTick
  (params (DeltaSeconds :type Float%20%28single-precision%29)))

(event Game|Damage|EventAnyDamage
  (params (Damage :type Float%20%28single-precision%29) (DamageType :type Damage%20Type%20Object%20Reference) (InstigatedBy :type Controller%20Object%20Reference) (DamageCauser :type Actor%20Object%20Reference))
  (bind _output_get (Variables|Default|SetHP (- (Variables|Default|GetHP) Damage)))
  (Development|PrintText (Utilities|Text|FormatText "Damaged {/Damage}, HP : {/HP}" Damage _output_get))
  (bind _output_get_2 (Variables|Default|SetIsDead (<= _output_get 0.0)))
  (if _output_get_2
    (Variables|Default|SetHp 0.0)
    (AI|Logic|StopLogic (Variables|/Script/AIModule.AIController|GetBrainComponent (AI|GetAIController self)) (Utilities|String|ToString(Boolean) _output_get_2))
    (Pawn|Components|CharacterMovement|DisableMovement (Variables|Character|GetCharacterMovement))
    (Utilities|FlowControl|DoOnce false
      (:Completed
        (Audio|PlaySoundatLocation "/Game/SCPEXODUS/Audio/SFX/Monsters_SFX/Kraken/SFX_Kraken_Death.SFX_Kraken_Death" (Transformation|GetActorLocation) "0, 0, 0" 1.0 1.0 0.0 0 0 0 0)
        (Components|Animation|PlayAnimation (Variables|Character|GetMesh) "/Game/SCPEXODUS/Characters/Kraken/Animations/KRAKEN_death.KRAKEN_death" false)
        (Utilities|FlowControl|Delay 1e+01)
        (Actor|DestroyActor)))))

(fn ConstructionScript)