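; BP_Enemy_Snork is an AI enemy character that runs the BT_Enemy_Snork behavior tree on BeginPlay.
; AnyDamage subtracts HP, prints a debug message and adds a particle component.
; At zero HP it stops AI logic and movement, then once plays death sound and animation before destroying itself after a delay.
; A MeleeAttack event plays the attack montage, and a disconnected ragdoll chain remains unused.
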(event Custom|MeleeAttack
  (Animation|Montage|PlayMontage (Variables|Character|GetMesh) "/Game/SCPEXODUS/Characters/Monster_Snork/Animation/SnorkAttackMontage.SnorkAttackMontage"))

(event EventBeginPlay
  (if (not (Variables|Default|GetIsDead))
    (AI|RunBehaviorTree (AI|GetAIController self) "/Game/SCPEXODUS/Blueprints/BT_Enemy_Snork.BT_Enemy_Snork")))

(event Collision|EventActorBeginOverlap
  (params (OtherActor :type Actor%20Object%20Reference)))

(event EventTick
  (params (DeltaSeconds :type Float%20%28single-precision%29)))

(event Game|Damage|EventAnyDamage
  (params (Damage :type Float%20%28single-precision%29) (DamageType :type Damage%20Type%20Object%20Reference) (InstigatedBy :type Controller%20Object%20Reference) (DamageCauser :type Actor%20Object%20Reference))
  (bind _mesh (Variables|Character|GetMesh))
  (bind _output_get (Variables|Default|SetHP (- (Variables|Default|GetHP) Damage)))
  (Development|PrintText (Utilities|Text|FormatText "Damaged {/Damage}, HP : {/HP}" Damage _output_get))
  (AddComponent|AddParticleSystemComponent false)
  (if (<= _output_get 0.0)
    (bind _output_get_2 (Variables|Default|SetIsDead true))
    (Variables|Default|SetHP 0.0)
    (AI|Logic|StopLogic (Variables|/Script/AIModule.AIController|GetBrainComponent (AI|GetAIController self)) (Utilities|String|ToString(Boolean) _output_get_2))
    (Pawn|Components|CharacterMovement|DisableMovement (Variables|Character|GetCharacterMovement))
    (Utilities|FlowControl|DoOnce false
      (:Completed
        (Audio|PlaySoundatLocation "/Game/SCPEXODUS/Audio/SFX/Monsters_SFX/Snork/SFX_Snork_Death_Cue.SFX_Snork_Death_Cue" (Transformation|GetActorLocation) "0, 0, 0" 1.0 1.0 0.0 0 0 0 0)
        (Components|Animation|PlayAnimation _mesh "/Game/SCPEXODUS/Characters/Monster_Snork/Animation/AS_Death_Snork.AS_Death_Snork" false)
        (Collision|SetCollisionEnabled _mesh "QueryAndPhysics")
        (Utilities|FlowControl|Delay 3.0)
        (Actor|DestroyActor)))))

(fn ConstructionScript)