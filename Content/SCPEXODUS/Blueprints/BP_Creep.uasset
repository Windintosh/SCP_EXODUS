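; BP_Creep is an AI-controlled enemy character with health and a melee attack.
; On BeginPlay it starts the BT_Creep behavior tree on its AI controller, and its MeleeAttack event plays an attack montage.
; Incoming damage lowers HP and prints a debug readout.
; At zero HP it stops AI logic and movement, then plays a death animation once and destroys itself after a short delay.
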(event Custom|MeleeAttack
  (Animation|Montage|PlayMontage (Variables|Character|GetMesh) "/Game/SCPEXODUS/Characters/Monster_Snork/Animation/SnorkAttackMontage.SnorkAttackMontage"))

(event EventBeginPlay
  (if (not (Variables|Default|GetIsDead))
    (AI|RunBehaviorTree (AI|GetAIController self) "/Game/SCPEXODUS/Blueprints/BT_Creep.BT_Creep")))

(event Collision|EventActorBeginOverlap
  (params (OtherActor :type Actor%20Object%20Reference)))

(event EventTick
  (params (DeltaSeconds :type Float%20%28single-precision%29)))

(event Game|Damage|EventAnyDamage
  (params (Damage :type Float%20%28single-precision%29) (DamageType :type Damage%20Type%20Object%20Reference) (InstigatedBy :type Controller%20Object%20Reference) (DamageCauser :type Actor%20Object%20Reference))
  (bind _output_get (Variables|Default|SetHP (- (Variables|Default|GetHP) Damage)))
  (Development|PrintText (Utilities|Text|FormatText "Damaged {/Damage}, HP : {/HP}" Damage _output_get))
  (bind _output_get_2 (Variables|Default|SetIsDead (<= _output_get 0.0)))
  (if _output_get_2
    (Variables|Default|SetHp 0.0)
    (AI|Logic|StopLogic (Variables|/Script/AIModule.AIController|GetBrainComponent (AI|GetAIController self)) (Utilities|String|ToString(Boolean) _output_get_2))
    (Pawn|Components|CharacterMovement|DisableMovement (Variables|Character|GetCharacterMovement))
    (Utilities|FlowControl|DoOnce false
      (:Completed
        (Components|Animation|PlayAnimation (Variables|Character|GetMesh) "/Game/SCPEXODUS/Characters/Monster_Creep/Anim/Creep_Death.Creep_Death" false)
        (Utilities|FlowControl|Delay 3.0)
        (Actor|DestroyActor)))))

(fn ConstructionScript)